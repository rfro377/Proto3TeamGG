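; Interactable distraction actor that can be switched on and off as a stimulus for AI perception.
; Its AI perception stimuli source is set inactive on BeginPlay, after the parent logic runs.
; Each Interact call toggles the source's active state without resetting it.
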(event EventBeginPlay
  (|CallParentFunction)
  (Components|Activation|SetActive (Variables|Default|GetAIPerceptionStimuliSource) false false))

(event Collision|EventActorBeginOverlap
  (params (OtherActor :type Actor%20Object%20Reference))
  (|CallParentFunction OtherActor) ; This node is disabled and will not be called.\nDrag off pins to build functionality.
)

(event EventTick
  (params (DeltaSeconds :type Float%20%28single-precision%29)))

(fn ConstructionScript
  (|CallParentFunction))

(fn Interact
  (bind _aiperceptionstimulisource (Variables|Default|GetAIPerceptionStimuliSource))
  (Components|Activation|SetActive _aiperceptionstimulisource (not (Components|Activation|IsActive _aiperceptionstimulisource)) false))