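; BP_TaskZone_Toys is a task zone in a ghost game that tracks progress on a toy task.
; It registers its task name with BP_GhostGameMode on BeginPlay.
; Each BP_Possessable1 overlap adds a quarter to progress; the RequiredItem comparison has no effect.
; Tick pushes progress to the HUD widget and, once full, marks the task done and calls FinishTask once on the game mode.
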(event OnComponentBeginOverlap(Collision)
  (params (OverlappedComponent :type Primitive%20Component%20Object%20Reference) (OtherActor :type Actor%20Object%20Reference) (OtherComp :type Primitive%20Component%20Object%20Reference) (OtherBodyIndex :type Integer) (bFromSweep :type Boolean) (SweepResult :type Hit%20Result%20Structure%20%28by%20ref%29))
  (bind _toyprogress (Variables|Default|GetToyProgress))
  (bind _asbp_possessable_1 (Utilities|Casting|CastToBP_Possessable1 OtherActor))
  (Utilities|ManipulateFloatInternal _toyprogress (+ _toyprogress 0.25)
    (:%20%20
      (if (and (Utilities|Enum|Equal(Enum) (Variables|/Game/Blueprint/BP_Possessable1.BP_Possessable1_C|GetItemType _asbp_possessable_1) (Variables|Default|GetRequiredItem)) false)
        _))))

(event Collision|EventActorBeginOverlap
  (params (OtherActor :type Actor%20Object%20Reference)))

(event EventBeginPlay
  (bind _asbp_ghost_game_mode (Utilities|Casting|CastToBP_GhostGameMode (Game|GetGameMode)))
  (Utilities|Array|Add (Variables|/Game/Maps/GamemOde/BP_GhostGameMode.BP_GhostGameMode_C|GetActiveTasks _asbp_ghost_game_mode) (Variables|Default|GetTaskName)))

(event EventTick
  (params (DeltaSeconds :type Float%20%28single-precision%29))
  (bind _toyprogress (Variables|Default|GetToyProgress))
  (bind _asghost_hud (Utilities|Casting|CastToGhostHUd (HUD|GetHUD (Game|GetPlayerController 0))))
  (Default|UpdateProgress (Variables|/Game/Maps/GamemOde/GhostHUd.GhostHUd_C|GetPlayerWidget _asghost_hud) (Variables|Default|GetTaskName) _toyprogress)
  (if (>= _toyprogress 1.0)
    (Variables|Default|SetTaskDone true)
    (Utilities|FlowControl|DoOnce false
      (:Completed
        (bind _asbp_ghost_game_mode (Utilities|Casting|CastToBP_GhostGameMode (Game|GetGameMode)))
        (Default|FinishTask _asbp_ghost_game_mode (Variables|Default|GetTaskName))))))

(fn ConstructionScript)