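; BP_TaskZone_DIshes is the dishwashing task zone, registering its task with BP_GhostGameMode on BeginPlay.
; Collision overlaps with BP_Possessable1 items, filtered by item type, adjust the dish count and progress or toggle a sponge flag.
; Tick sends progress as a fraction of 20 to the GhostHUd widget.
; At full progress it plays a washing sound every tick and finishes the task once through a DoOnce.
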(event OnComponentBeginOverlap(Collision)
  (params (OverlappedComponent :type Primitive%20Component%20Object%20Reference) (OtherActor :type Actor%20Object%20Reference) (OtherComp :type Primitive%20Component%20Object%20Reference) (OtherBodyIndex :type Integer) (bFromSweep :type Boolean) (SweepResult :type Hit%20Result%20Structure%20%28by%20ref%29))
  (bind _asbp_possessable_1 (Utilities|Casting|CastToBP_Possessable1 OtherActor))
  (Utilities|FlowControl|Sequence
    (:then_0
      (if (Utilities|Enum|Equal(Enum) (Variables|/Game/Blueprint/BP_Possessable1.BP_Possessable1_C|GetItemType _asbp_possessable_1) "NewEnumerator1")
        (Math|Integer|IncrementInt (Variables|Default|GetDishesInSink)
          (:%20%20
            (Math|Float|IncrementFloat (Variables|Default|GetCleaningProgress))))))
    (:then_1
      (if (Utilities|Enum|Equal(Enum) (Variables|/Game/Blueprint/BP_Possessable1.BP_Possessable1_C|GetItemType _asbp_possessable_1) "NewEnumerator5")
        (Variables|Default|SethasSponge true)
        (if (>= (Variables|Default|GetCleaningProgress) 1e+02)
          (Variables|Default|SetTaskDone true))))))

(event OnComponentEndOverlap(Collision)
  (params (OverlappedComponent :type Primitive%20Component%20Object%20Reference) (OtherActor :type Actor%20Object%20Reference) (OtherComp :type Primitive%20Component%20Object%20Reference) (OtherBodyIndex :type Integer))
  (bind _asbp_possessable_1 (Utilities|Casting|CastToBP_Possessable1 OtherActor))
  (Utilities|FlowControl|Sequence
    (:then_0
      (if (Utilities|Enum|Equal(Enum) (Variables|/Game/Blueprint/BP_Possessable1.BP_Possessable1_C|GetItemType _asbp_possessable_1) "NewEnumerator1")
        (Variables|Default|SetDishesInSink (- (Variables|Default|GetDishesInSink) 1))
        (Variables|Default|SetCleaningProgress (- (Variables|Default|GetCleaningProgress) 1.0))))
    (:then_1
      (if (Utilities|Enum|Equal(Enum) (Variables|/Game/Blueprint/BP_Possessable1.BP_Possessable1_C|GetItemType _asbp_possessable_1) "NewEnumerator5")
        (Variables|Default|SethasSponge false)))))

(event EventTick
  (params (DeltaSeconds :type Float%20%28single-precision%29))
  (bind _cleaningprogress (Variables|Default|GetCleaningProgress))
  (bind _returnvalue (/ _cleaningprogress 2e+01))
  (bind _asghost_hud (Utilities|Casting|CastToGhostHUd (HUD|GetHUD (Game|GetPlayerController 0))))
  (Default|UpdateProgress (Variables|/Game/Maps/GamemOde/GhostHUd.GhostHUd_C|GetPlayerWidget _asghost_hud) (Variables|Default|GetTaskName) _returnvalue)
  (if (>= _returnvalue 1.0)
    (Audio|PlaySound2D "/Game/Sounds/washing_dishes_86204.washing_dishes_86204" 1.0 1.0 0.0 0 0)
    (Utilities|FlowControl|DoOnce false
      (:Completed
        (Variables|Default|SetTaskDone true)
        (bind _asbp_ghost_game_mode (Utilities|Casting|CastToBP_GhostGameMode (Game|GetGameMode)))
        (Default|FinishTask _asbp_ghost_game_mode (Variables|Default|GetTaskName))))))

(event Collision|EventActorBeginOverlap
  (params (OtherActor :type Actor%20Object%20Reference)))

(event EventBeginPlay
  (bind _asbp_ghost_game_mode (Utilities|Casting|CastToBP_GhostGameMode (Game|GetGameMode)))
  (Utilities|Array|Add (Variables|/Game/Maps/GamemOde/BP_GhostGameMode.BP_GhostGameMode_C|GetActiveTasks _asbp_ghost_game_mode) (Variables|Default|GetTaskName)))

(fn ConstructionScript)