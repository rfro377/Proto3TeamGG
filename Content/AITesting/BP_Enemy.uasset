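; BP_Enemy is an AI test enemy that moves toward the player when it sees them.
; Its PawnSensing component reports seen pawns, and only a BP_ThirdPersonCharacter sets IsSeeingPlayer, which this graph never clears.
; On each sighting it snaps to face the player with pitch zeroed, then uses AIMoveTo toward the player's current location rather than tracking the actor.
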(event OnSeePawn(PawnSensing)
  (params (Pawn :type Pawn%20Object%20Reference))
  (bind _asbp_third_person_character (Utilities|Casting|CastToBP_ThirdPersonCharacter Pawn))
  (Variables|Default|SetisSeeingPlayer? true)
  (Transformation|SetActorRotation (Math|Rotator|MakeRotator (.roll (Math|Rotator|FindLookatRotation (Transformation|GetActorLocation self) (Transformation|GetActorLocation _asbp_third_person_character))) 0.0 (.yaw (Math|Rotator|FindLookatRotation (Transformation|GetActorLocation self) (Transformation|GetActorLocation _asbp_third_person_character)))))
  (AI|AIMoveTo self (Transformation|GetActorLocation _asbp_third_person_character) 0 0.5 false))

(event EventBeginPlay)

(event Collision|EventActorBeginOverlap
  (params (OtherActor :type Actor%20Object%20Reference)))

(event EventTick
  (params (DeltaSeconds :type Float%20%28single-precision%29)))

(fn ConstructionScript)